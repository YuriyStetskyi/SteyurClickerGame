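; BP_SCGPlayerCharacter is the player character Blueprint, providing a custom mouse cursor and a debug check for interactable targets under it.
; BeginPlay shows the mouse and sets WBP_Cursor as player 0's default cursor widget.
; Each Tick runs a complex Visibility trace under the cursor and checks the hit actor for the Gameplay.Interactable.Player tag.
; A hit only prints a keyed "targeted" or "no" message; no interaction follows.
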(event `self.ReceiveBeginPlay`
  (bind _returnvalue (`GameplayStatics.GetPlayerController` 0))
  (set `PlayerController.bShowMouseCursor` true _returnvalue)
  (bind _returnvalue_2 (`|CreateWidget` "/Game/Game/UI/HUD/WBP_Cursor.WBP_Cursor_C" _returnvalue))
  (`PlayerController.SetMouseCursorWidget` _returnvalue "Default" _returnvalue_2))

(event `self.ReceiveTick`
  (params (DeltaSeconds :type "Float (single-precision)"))
  (bind (_hitresult _returnvalue) (`PlayerController.GetHitResultUnderCursorByChannel` (`GameplayStatics.GetPlayerController` 0) "TraceTypeQuery1" true))
  (if _returnvalue
    (bind _returnvalue_2 (message `GameplayTagAssetInterface.HasMatchingGameplayTag` (`.HitActor` (`GameplayStatics.BreakHitResult` _hitresult)) (struct :`TagName` "Gameplay.Interactable.Player")))
    (if _returnvalue_2
      (`KismetSystemLibrary.PrintString` "targeted" true true (struct :`G` 1.0 :`B` 0.086251 :`A` 1.0) 2.0 "-35")
      (else
        (`KismetSystemLibrary.PrintString` "no" true true (struct :`R` 1.0 :`B` 0.018926 :`A` 1.0) 2.0 "-35")))))

(fn `UserConstructionScript`)